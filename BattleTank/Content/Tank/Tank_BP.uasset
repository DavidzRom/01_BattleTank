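; Player tank Blueprint that handles camera aiming and firing.
; On BeginPlay it passes the Barrel and TankTurret components to SetBarrelReference and SetTurretReference.
; Aim axes rotate the camera rig, scaled by delta time: yaw on the azimuth gimbal, pitch on the spring arm, keeping the two rotations separate.
; The Fire action calls Fire; controller pitch and yaw input nodes are left unconnected.
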(event `self.ReceiveBeginPlay`
  (`self.SetBarrelReference` (`self.Barrel`))
  (`self.SetTurretReference` (`self.TankTurret`)))

(event `InputAxis|AImAzimuth`
  (params (AxisValue :type "Float (single-precision)"))
  ;[1 1 1] Camera Input binding
  (`SceneComponent.K2_AddLocalRotation` (`self.Aimuth Gimbal`) (`KismetMathLibrary.MakeRotator` 0.0 0.0 (* AxisValue (`GameplayStatics.GetWorldDeltaSeconds`) 100.0)) false false))

(event `InputAxis|AimElevation`
  (params (AxisValue :type "Float (single-precision)"))
  ;[1 1 1] Camera Input binding
  (`SceneComponent.K2_AddLocalRotation` (`self.SpringArm`) (`KismetMathLibrary.MakeRotator` 0.0 (* AxisValue (`GameplayStatics.GetWorldDeltaSeconds`) 100.0)) false false))

(event `InputAction|Fire`
  (params (Key :type "Key Structure" :default "AnyKey"))
  ;[1 1 1] Camera Input binding
  (:`Pressed`
    (`self.Fire`)))

(fn `UserConstructionScript`)